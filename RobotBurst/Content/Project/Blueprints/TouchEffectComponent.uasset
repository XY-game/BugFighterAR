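; Actor component that shows touch ripple effects on screen at a given screen position.
; On BeginPlay it creates a small pool of TouchRipple widgets for the first player and adds them to the viewport.
; ShowTouchEffect picks the first pooled ripple that is not visible and triggers it at the position, doing nothing when all are in use.
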(event `self.ReceiveBeginPlay`
  (for _ (range 6)
    (bind _returnvalue (`|CreateWidget` "/Game/Project/Blueprints/TouchRipple.TouchRipple_C" (`GameplayStatics.GetPlayerController` 0)))
    (`UserWidget.AddToViewport` _returnvalue 0)
    (`KismetArrayLibrary.Array_Add` (`self.RippleEffectPool`) _returnvalue)))

(fn `GetUnusedRipple`
  (returns (RippleInstance :type "/Game/Project/Blueprints/TouchRipple Object Reference"))
  (for _array_element (`self.RippleEffectPool`)
    (if (not (`Widget.IsVisible` _array_element))
      (return _array_element)))
  (return null))

(fn `ShowTouchEffect`
  (params (ScreenPosition :type "Vector2D Structure"))
  (locals (Ripple :type "/Game/Project/Blueprints/TouchRipple Object Reference"))
  (bind _rippleinstance (`self.GetUnusedRipple`))
  (if (`KismetSystemLibrary.IsValid` _rippleinstance)
    (`/Game/Project/Blueprints/TouchRipple.TriggerRipple` _rippleinstance ScreenPosition)))